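; Behavior tree task that picks an AI Bomberman's move target, either chasing the player or fleeing a nearby bomb.
; It scans all BP_Bomb actors for the one closest to the controlled pawn and compares that distance to MaxDistanceWithBomb.
; It writes the player's location or the character's GetFleeLocation result to the MoveLocation blackboard key, then finishes after a short delay.
; The cached nearest distance resets only on the flee branch.
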(event `self.ReceiveExecuteAI`
  (params (OwnerController :type "AIController Object Reference") (ControlledPawn :type "Pawn Object Reference"))
  (set `self.Controlled Pawn` ControlledPawn)
  (set `self.ActorLocation` (`Actor.K2_GetActorLocation` ControlledPawn))
  (bind _outactors (`GameplayStatics.GetAllActorsOfClass` "/Game/Blueprint/BP_Bomb.BP_Bomb_C"))
  (for _array_element _outactors
    (bind _returnvalue (`Actor.K2_GetActorLocation` _array_element))
    (bind _returnvalue_2 (`KismetMathLibrary.Vector_Distance` _returnvalue (`self.ActorLocation`)))
    (if (< _returnvalue_2 (`self.NearestDistance`))
      (set `self.NearestDistance` _returnvalue_2)
      (set `self.LocNearestDistance` _returnvalue)
      (set `self.CloserBomb` _array_element)))
  (if (> (`self.NearestDistance`) (`self.maxDistanceWithBomb`))
    (`self.RunToPlayer`)
    (else
      (`self.RunFromBomb`)))
  (`KismetSystemLibrary.Delay` 0.5)
  (`self.FinishExecute` true))

(event `RunToPlayer`
  (`BTFunctionLibrary.SetBlackboardValueAsVector` (`self.MoveLocation`) (`Actor.K2_GetActorLocation` (`GameplayStatics.GetPlayerCharacter` 0))))

(event `RunFromBomb`
  (bind _asbomberman_character (cast `BombermanCharacter` (`self.Controlled Pawn`)))
  (bind _returnvalue (`BombermanCharacter.GetFleeLocation` _asbomberman_character (`Actor.K2_GetActorLocation` (`self.CloserBomb`))))
  (`BTFunctionLibrary.SetBlackboardValueAsVector` (`self.MoveLocation`) _returnvalue)
  (set `self.NearestDistance` 20000.0))