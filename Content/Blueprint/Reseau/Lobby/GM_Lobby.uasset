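; GM_Lobby is the lobby game mode, keeping the lobby's player count up to date as players join and leave.
; On PostLogin it casts the game state to GS_Lobby and calls UpdateNbPlayer with NbPlayer plus one.
; On Logout it does the same with NbPlayer minus one, leaving storage of the count to the game state.
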(event `self.K2_PostLogin`
  (params (NewPlayer :type "PlayerController Object Reference"))
  (bind _asgs_lobby (cast `/Game/Blueprint/Reseau/Lobby/GS_Lobby` (`GameplayStatics.GetGameState`)))
  (`/Game/Blueprint/Reseau/Lobby/GS_Lobby.UpdateNbPlayer` _asgs_lobby (+ (`/Game/Blueprint/Reseau/Lobby/GS_Lobby.NbPlayer` _asgs_lobby) 1)))

(event `self.K2_OnLogout`
  (params (ExitingController :type "Controller Object Reference"))
  (bind _asgs_lobby (cast `/Game/Blueprint/Reseau/Lobby/GS_Lobby` (`GameplayStatics.GetGameState`)))
  (`/Game/Blueprint/Reseau/Lobby/GS_Lobby.UpdateNbPlayer` _asgs_lobby (- (`/Game/Blueprint/Reseau/Lobby/GS_Lobby.NbPlayer` _asgs_lobby) 1)))

(fn `UserConstructionScript`)