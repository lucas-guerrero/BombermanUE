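; Player controller for a networked match, handling death and the end of the game.
; It clears all widgets on begin play, and Dead switches the view to the first BP_GameCamera in the level.
; Tick polls the GSGame state; when the game can finish, it calls Finish with whether a pawn is still possessed.
; After a short delay, authority destroys the session, and both authority and clients open MainMenu.
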(event `self.ReceiveBeginPlay`
  (`WidgetLayoutLibrary.RemoveAllWidgets`))

(event `self.ReceiveTick`
  (params (DeltaSeconds :type "Float (single-precision)"))
  (bind _asgsgame (cast `GSGame` (`GameplayStatics.GetGameState`)))
  (bind _returnvalue (`GSGame.CanFinish` _asgsgame))
  (if _returnvalue
    (`self.Finish` (`KismetSystemLibrary.IsValid` (`self.K2_GetPawn`)))
    (`KismetSystemLibrary.Delay` 5.0)
    (if (`self.HasAuthority`)
      (`DestroySessionCallbackProxy.DestroySession` self
        (:`OnSuccess`
          _)
        (:`OnFailure`
          _)))
    (`GameplayStatics.OpenLevel` "MainMenu")))

(fn `Dead`
  (bind _outactors (`GameplayStatics.GetAllActorsOfClass` "/Game/Blueprint/Gameplay/BP_GameCamera.BP_GameCamera_C"))
  (`self.SetViewTargetWithBlend` (`|GetArrayItem` _outactors)))

(fn `UserConstructionScript`)