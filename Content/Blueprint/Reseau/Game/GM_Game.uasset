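; GM_Game is the networked match's game mode, which places players at numbered starts and fills the remaining slots, up to four, with bots.
; ChoosePlayerStart increments a player counter, passes it to GSGame's SetNbPlayer and returns the start named after that number.
; One second after BeginPlay, it spawns a BP_Bot at each remaining numbered start and hands it the level's BP_GenerateLevel actor.
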(event `self.ReceiveBeginPlay`
  (`KismetSystemLibrary.Delay` 1.0)
  (for _index (range (+ (`self.IndexPlayer`) 1) 5)
    (bind _returnvalue (`|SpawnActorFromClass` "/Game/Blueprint/Charactere/BP_Bot.BP_Bot_C" (`self.GetTransform` (`self.K2_FindPlayerStart` (`GameplayStatics.GetPlayerController` 0) (`KismetStringLibrary.Conv_IntToString` _index))) "Undefined" "OverrideRootScale" null null))
    (bind _outactors (`GameplayStatics.GetAllActorsOfClass` "/Game/Blueprint/Gameplay/BP_GenerateLevel.BP_GenerateLevel_C"))
    (set `BombermanCharacter.GeneratedLevel` (`|GetArrayItem` _outactors) _returnvalue)))

(fn `ChoosePlayerStart`
  (params (Player :type "Controller Object Reference"))
  (returns (ReturnValue :type "Actor Object Reference"))
  (bind _asgsgame (cast `GSGame` (`GameplayStatics.GetGameState`)))
  (bind _result (`/Engine/EditorBlueprintResources/StandardMacros.IncrementInt` (`self.IndexPlayer`))
    (:`  `
      (`GSGame.SetNbPlayer` _asgsgame _result)
      (return (`self.K2_FindPlayerStart` Player (`KismetStringLibrary.Conv_IntToString` (`self.IndexPlayer`)))))))

(fn `UserConstructionScript`)